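; Quest manager actor that shows the current quest text on screen and lets the player skip quests by holding Space Bar.
; On BeginPlay it creates the quest text and skip progress widgets and binds text updates, hiding the quest text when empty.
; A hold timer drives the progress bar each tick; on completion, if the quest text is visible, it hides it, calls SkipQuests and destroys the actor.
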(event Custom|UpdateUIText
  (params (Text :type String) (bIsNewQuest :type Boolean))
  (bind _questui (Variables|Default|GetQuestUI))
  (Default|UpdateUIText _questui Text bIsNewQuest)
  (if (Utilities|Array|IsEmpty Text)
    (Widget|SetVisibility _questui "Hidden")))

(event Custom|OnSpaceBarHeld
  (bind _questui (Variables|Default|GetQuestUI))
  ;[1 1 1] Skip Quest on holding Space Bar
  (Utilities|IsValid _questui
    (:Is%20Valid
      (if (Widget|IsVisible _questui)
        (Widget|SetVisibility _questui "Hidden")
        (Class|QuestManager|SkipQuests)
        (Actor|DestroyActor)))))

(event EventBeginPlay
  (bind _returnvalue (Game|GetPlayerController 0))
  (Input|EnableInput _returnvalue)
  (bind _returnvalue_2 (UserInterface|CreateWidget "/Game/UI/Quest/BP_UI_QuestSkipProgress.BP_UI_QuestSkipProgress_C" _returnvalue))
  (bind _output_get (Variables|Default|SetQuestSkipUI _returnvalue_2))
  (UserInterface|Viewport|AddtoViewport _output_get 0)
  (bind _returnvalue_3 (UserInterface|CreateWidget "/Game/UI/Quest/BP_UI_QuestText.BP_UI_QuestText_C" _returnvalue))
  (bind _output_get_2 (Variables|Default|SetQuestUI _returnvalue_3))
  (UserInterface|Viewport|AddtoViewport _output_get_2 0)
  (EventDispatchers|BindEventtoOnUITextChange (delegate Custom|UpdateUIText)))

(event EventTick
  (params (DeltaSeconds :type Float%20%28single-precision%29))
  (bind _questskipui (Variables|Default|GetQuestSkipUI))
  (bind _spacebartimer (Variables|Default|GetSpaceBarTimer))
  (bind _returnvalue (Class|KismetSystemLibrary|GetTimerElapsedTimeHandle _spacebartimer))
  (bind _progressbar_91 (Variables|/Game/UI/Quest/BP_UI_QuestSkipProgress.BP_UI_QuestSkipProgress_C|GetProgressBar_91 _questskipui))
  (|CallParentFunction DeltaSeconds)
  (if (Utilities|Time|IsTimerActivebyHandle _spacebartimer)
    (Progress|SetPercent _progressbar_91 (/ _returnvalue (+ _returnvalue (Utilities|Time|GetTimerRemainingTimebyHandle _spacebartimer))))
    (else
      (Progress|SetPercent _progressbar_91 0.0))))

(event Input|KeyboardEvents|SpaceBar
  (params (Key :type Key%20Structure :default "None"))
  ;[1 1 1] Skip Quest on holding Space Bar
  (:Pressed
    (bind _returnvalue (Utilities|Time|SetTimerbyEvent (delegate Custom|OnSpaceBarHeld) (Variables|Default|GetHoldTimeForSkipQuest)))
    (Variables|Default|SetSpaceBarTimer _returnvalue))
  (:Released
    (Utilities|Time|ClearandInvalidateTimerbyHandle (Variables|Default|GetSpaceBarTimer))))

(fn ConstructionScript)