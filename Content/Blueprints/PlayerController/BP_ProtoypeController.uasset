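; Prototype player controller for an RTS-style game, handling pause, input mode and unit selection.
; Locks the mouse in Game and UI mode on begin play, and a pause input toggles game pause and the UI_PauseMenu widget.
; Idle worker, warrior, spitter and tank shortcuts delegate to BP_GP3GameMode.
; Selection functions maintain a unique unit list and each unit's selected state; SetCameraLocation is an empty stub.
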(event Custom|SetCameraLocation
  (params (Location :type Vector)))

(event Input|EnhancedActionEvents|EnhancedInputActionIA_Pause
  (params (ActionValue :type Boolean) (ElapsedSeconds :type Float%20%28double-precision%29) (TriggeredSeconds :type Float%20%28double-precision%29) (InputAction :type Input%20Action%20Object%20Reference :default "/Game/Settings/Inputs/IA_Pause.IA_Pause"))
  ;[1 1 1] Press P = pause
  (:Started
    (if (not (Variables|Default|GetIsPauseOpen))
      (Variables|Default|SetIsPauseOpen true)
      (bind _returnvalue (UserInterface|CreateWidget "/Game/UI/Menus/UI_PauseMenu.UI_PauseMenu_C" self))
      (Variables|Default|SetPauseMenuWidget _returnvalue)
      (Game|SetGamePaused true)
      (UserInterface|Viewport|AddtoViewport _returnvalue 0)
      (else
        (Variables|Default|SetIsPauseOpen false)
        (Widget|RemovefromParent (Variables|Default|GetPauseMenuWidget))
        (Game|SetGamePaused false)))))

(event Input|EnhancedActionEvents|EnhancedInputActionIA_SelectIdleWorkers
  (params (ActionValue :type Boolean) (ElapsedSeconds :type Float%20%28double-precision%29) (TriggeredSeconds :type Float%20%28double-precision%29) (InputAction :type Input%20Action%20Object%20Reference :default "/Game/Settings/Inputs/IA_SelectIdleWorkers.IA_SelectIdleWorkers"))
  (:Completed
    (bind _asbp_gp3game_mode (Utilities|Casting|CastToBP_GP3GameMode (Game|GetGameMode)))
    (Default|SelectIdleWorkers _asbp_gp3game_mode)))

(event Input|EnhancedActionEvents|EnhancedInputActionIA_SelectIdleWarriors
  (params (ActionValue :type Boolean) (ElapsedSeconds :type Float%20%28double-precision%29) (TriggeredSeconds :type Float%20%28double-precision%29) (InputAction :type Input%20Action%20Object%20Reference :default "/Game/Settings/Inputs/IA_SelectIdleWarriors.IA_SelectIdleWarriors"))
  (:Completed
    (bind _asbp_gp3game_mode (Utilities|Casting|CastToBP_GP3GameMode (Game|GetGameMode)))
    (Default|SelectIdleWarriors _asbp_gp3game_mode)))

(event Input|EnhancedActionEvents|EnhancedInputActionIA_SelectIdleSpitters
  (params (ActionValue :type Boolean) (ElapsedSeconds :type Float%20%28double-precision%29) (TriggeredSeconds :type Float%20%28double-precision%29) (InputAction :type Input%20Action%20Object%20Reference :default "/Game/Settings/Inputs/IA_SelectIdleSpitters.IA_SelectIdleSpitters"))
  (:Completed
    (bind _asbp_gp3game_mode (Utilities|Casting|CastToBP_GP3GameMode (Game|GetGameMode)))
    (Default|SelectIdleSpitters _asbp_gp3game_mode)))

(event Input|EnhancedActionEvents|EnhancedInputActionIA_SelectIdleTanks
  (params (ActionValue :type Boolean) (ElapsedSeconds :type Float%20%28double-precision%29) (TriggeredSeconds :type Float%20%28double-precision%29) (InputAction :type Input%20Action%20Object%20Reference :default "/Game/Settings/Inputs/IA_SelectIdleTanks.IA_SelectIdleTanks"))
  (:Completed
    (bind _asbp_gp3game_mode (Utilities|Casting|CastToBP_GP3GameMode (Game|GetGameMode)))
    (Default|SelectIdleTanks _asbp_gp3game_mode)))

(event EventBeginPlay
  (Input|SetInputModeGameandUI self 0 "LockAlways" false false))

(fn ConstructionScript)

(fn AddUnittoSelection
  (params (UnitBase :type Unit%20Base%20Object%20Reference))
  (Utilities|Array|AddUnique (Variables|Default|GetUnitSelection) UnitBase)
  (Default|IsSelected UnitBase true))

(fn RemoveUnitfromSelection
  (params (UnitBase :type Unit%20Base%20Object%20Reference))
  (Utilities|Array|RemoveItem (Variables|Default|GetUnitSelection) UnitBase)
  (Default|IsSelected UnitBase false))

(fn ClearUnitSelection
  (for _array_element (Variables|Default|GetUnitSelection)
    (Default|IsSelected _array_element false))
  (Utilities|Array|Clear (Variables|Default|GetUnitSelection)))