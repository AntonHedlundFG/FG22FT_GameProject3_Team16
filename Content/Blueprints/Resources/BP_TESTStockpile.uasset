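; BP_TESTStockpile is a test resource stockpile that units pick up resources from by overlapping its box.
; On overlap, it casts the actor to BP_UnitBase, increments CarryingResource and refreshes the unit frame UI.
; It then writes its EAction value to the EActionEnum key on the unit's AI blackboard, intended to switch the ant's behavior tree to collecting.
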(event OnComponentBeginOverlap(Box)
  (params (OverlappedComponent :type Primitive%20Component%20Object%20Reference) (OtherActor :type Actor%20Object%20Reference) (OtherComp :type Primitive%20Component%20Object%20Reference) (OtherBodyIndex :type Integer) (bFromSweep :type Boolean) (SweepResult :type Hit%20Result%20Structure%20%28by%20ref%29))
  ;[1 1 1] Sets "Carrying Resource" variable in Unit Base to 1.
  (bind _asbp_unit_base (Utilities|Casting|CastToBP_UnitBase OtherActor))
  (Variables|Default|SetAs%20BP%20Unit%20Base _asbp_unit_base)
  (Variables|/Game/Blueprints/Actors/BP_UnitBase.BP_UnitBase_C|SetCarryingResource (Variables|Default|GetAs%20BP%20Unit%20Base) (+ (Variables|/Game/Blueprints/Actors/BP_UnitBase.BP_UnitBase_C|GetCarryingResource (Variables|Default|GetAs%20BP%20Unit%20Base)) 1))
  ;[1 1 1] Updated UI on Unit
  (Default|UpdateUnitFrame (Variables|Default|GetAs%20BP%20Unit%20Base))
  ;[1 1 1] Sets the bahavior of ant to "Collecting" in Behaviour Tree through Enum.
  (AI|Components|Blackboard|SetValueasEnum (Variables|/Script/AIModule.AIController|GetBlackboard (AI|GetAIController OtherActor)) (Utilities|Name|MakeLiteralName "EActionEnum") (Variables|Default|GetEAction)))

(fn ConstructionScript)