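; Enemy tank unit that fights AI-chosen targets, takes damage and identifies itself as a hostile unit to selection queries.
; Damage adopts the attacker as Blackboard target if none is set, updates the health component and widget, and destroys the unit on death.
; Attack turns toward the controller's target, waits, range-checks using the stats asset, then deals damage when the montage completes.
; Shortly after BeginPlay, it unregisters itself as a sight stimulus.
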(event Custom|Attack
  ;[1 1 1] Attack
  (bind _asai_enemy_unit_controller (Utilities|Casting|CastToAI_EnemyUnitController (AI|GetAIController self)))
  (Transformation|SetActorRotation (Math|Rotator|MakeRotator 0.0 0.0 (.yaw (Math|Interpolation|RInterpTo (Transformation|GetActorRotation) (Math|Rotator|FindLookatRotation (Transformation|GetActorLocation) (Transformation|GetActorLocation (Variables|/Game/AI/EnemyAnts/AI_EnemyUnitController.AI_EnemyUnitController_C|GetTarget%20Actor _asai_enemy_unit_controller))) (Utilities|Time|GetWorldDeltaSeconds) 2e+01))))
  (Utilities|FlowControl|Delay (Variables|Default|GetAttack%20Speed))
  (bind _returnvalue (Class|UnitStatsAsset|GetRange (Variables|/Game/Blueprints/Health_Damage/BP_HealthComponent.BP_HealthComponent_C|GetStats%20Asset (Variables|Default|GetBP_HealthComponent))))
  (if (and (Utilities|IsValid (Variables|/Game/AI/EnemyAnts/AI_EnemyUnitController.AI_EnemyUnitController_C|GetTarget%20Actor _asai_enemy_unit_controller)) (<= (Transformation|GetDistanceTo (Variables|/Game/AI/EnemyAnts/AI_EnemyUnitController.AI_EnemyUnitController_C|GetTarget%20Actor _asai_enemy_unit_controller)) _returnvalue))
    (Animation|Montage|PlayMontage (Variables|Character|GetMesh) (Variables|Default|GetMontage%20to%20Play_0)
      (:OnCompleted
        (bind _returnvalue_2 (Class|UnitStatsAsset|GetDamage (Variables|/Game/Blueprints/Health_Damage/BP_HealthComponent.BP_HealthComponent_C|GetStats%20Asset (Variables|Default|GetBP_HealthComponent))))
        (Class|BPIDamageable|OnDamage(Message) (Variables|/Game/AI/EnemyAnts/AI_EnemyUnitController.AI_EnemyUnitController_C|GetTarget%20Actor _asai_enemy_unit_controller) _returnvalue_2 self)))))

(event EventBeginPlay
  (|CallParentFunction)
  ;[0 0 0] Disable Player AI Perception
  (Utilities|FlowControl|Delay 0.05)
  (Class|AIPerceptionStimuliSourceComponent|UnregisterfromSense (Variables|Default|GetAIPerceptionStimuliSource) "/Script/AIModule.AISense_Sight"))

(event EventTick
  (params (DeltaSeconds :type Float%20%28single-precision%29)))

(event EventOnDamage
  (params (Damage :type Float%20%28double-precision%29) (AttackingActor :type Actor%20Object%20Reference))
  (bind _bp_healthcomponent (Variables|Default|GetBP_HealthComponent))
  (bind _bp_healthcomponent_2 (Variables|Default|GetBP_HealthComponent))
  ;[1 1 1] Recieving Damage
  (if (Utilities|IsValid (Variables|Default|GetTargetActor))
    _
    (else
      (bind _output_get (Variables|Default|SetTargetActor AttackingActor))
      (AI|Components|Blackboard|SetValueasObject (AI|GetBlackboard 0) (Utilities|Name|MakeLiteralName "TargetActor") _output_get)))
  (Default|ChangeHealth _bp_healthcomponent_2 Damage)
  (Rendering|SetVisibility (Variables|Default|GetUnitFrame) true false)
  (bind _asui_enemy_health (Utilities|Casting|CastToUI_EnemyHealth (UserInterface|GetUserWidgetObject (Variables|Default|GetUnitFrame))))
  (Default|UpdateHealth _asui_enemy_health (Variables|/Game/Blueprints/Health_Damage/BP_HealthComponent.BP_HealthComponent_C|GetCurrentHealth _bp_healthcomponent) (Variables|/Game/Blueprints/Health_Damage/BP_HealthComponent.BP_HealthComponent_C|GetMaxHealth _bp_healthcomponent))
  (if (not (Variables|/Game/Blueprints/Health_Damage/BP_HealthComponent.BP_HealthComponent_C|GetisAlive _bp_healthcomponent_2))
    (Actor|DestroyActor)))

(fn ConstructionScript
  (|CallParentFunction))

(fn GetSelectorType
  (return "STT_HOSTILE_UNIT"))