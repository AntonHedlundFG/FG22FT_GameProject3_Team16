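; Queen enemy unit, a child Blueprint whose death triggers the end of the game.
; Shortly after BeginPlay it unregisters its stimuli source from AI sight.
; Damage updates the health component and reveals the unit frame's health bar.
; On death, a one-time guard plays a fanfare and adds a fade screen widget, then opens the end scene after a delay.
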(event EventBeginPlay
  (|CallParentFunction)
  ;[0 0 0] Disable Player AI Perception
  (Utilities|FlowControl|Delay 0.05)
  (Class|AIPerceptionStimuliSourceComponent|UnregisterfromSense (Variables|Default|GetAIPerceptionStimuliSource) "/Script/AIModule.AISense_Sight"))

(event Collision|EventActorBeginOverlap
  (params (OtherActor :type Actor%20Object%20Reference))
  (|CallParentFunction OtherActor) ; This node is disabled and will not be called.\nDrag off pins to build functionality.
)

(event EventTick
  (params (DeltaSeconds :type Float%20%28single-precision%29))
  (|CallParentFunction DeltaSeconds) ; This node is disabled and will not be called.\nDrag off pins to build functionality.
)

(event EventOnDamage
  (params (Damage :type Float%20%28double-precision%29) (AttackingActor :type Actor%20Object%20Reference))
  (bind _bp_healthcomponent (Variables|Default|GetBP_HealthComponent))
  (bind _bp_healthcomponent_2 (Variables|Default|GetBP_HealthComponent))
  ;[1 1 1] Take Damage
  (Default|ChangeHealth _bp_healthcomponent_2 Damage)
  (Rendering|SetVisibility (Variables|Default|GetUnitFrame) true false)
  (bind _asui_enemy_health (Utilities|Casting|CastToUI_EnemyHealth (UserInterface|GetUserWidgetObject (Variables|Default|GetUnitFrame))))
  (Default|UpdateHealth _asui_enemy_health (Variables|/Game/Blueprints/Health_Damage/BP_HealthComponent.BP_HealthComponent_C|GetCurrentHealth _bp_healthcomponent) (Variables|/Game/Blueprints/Health_Damage/BP_HealthComponent.BP_HealthComponent_C|GetMaxHealth _bp_healthcomponent))
  (if (not (Variables|/Game/Blueprints/Health_Damage/BP_HealthComponent.BP_HealthComponent_C|GetisAlive _bp_healthcomponent_2))
    (if (not (Variables|Default|GetHasPlayed))
      (Variables|Default|SetHasPlayed true)
      (Audio|Components|Audio|Play (Variables|Default|GetFanfare) 0.0)
      (bind _returnvalue (UserInterface|CreateWidget "/Game/Blueprints/LoadingScreen/W_FadeScreen.W_FadeScreen_C"))
      (UserInterface|Viewport|AddtoViewport _returnvalue 0)
      (Utilities|FlowControl|Delay 6.0)
      (Game|OpenLevel(byObjectReference) "/Game/Scenes/GameScene/EndScene.EndScene"))))

(fn ConstructionScript
  (|CallParentFunction))