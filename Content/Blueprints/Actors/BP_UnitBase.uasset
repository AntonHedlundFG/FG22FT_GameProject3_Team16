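; Base Blueprint for RTS ant units, handling selection feedback, move and target orders, flag indicators, sounds and quest completion.
; Player units bind C++ selection and targeting events and write orders to the AI Blackboard, while non-player units get a red decal.
; A looping timer refreshes walk speed from the stats asset.
; Player units also run staggered, timed sphere-overlap checks that trigger short Tick-driven pushes away from nearby units.
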(event Custom|SetDecalVisibility
  (params (State :type Boolean)))

(event Custom|SpeedUpdate
  ;[1 1 1] Updates Movespeed from the UnitStats data asset on a regular basis
  (bind _returnvalue (Class|UnitStatsAsset|GetMoveSpeed (Variables|/Game/Blueprints/Health_Damage/BP_HealthComponent.BP_HealthComponent_C|GetStats%20Asset (Variables|Default|GetBP_HealthComponent))))
  (Variables|/Script/Engine.CharacterMovementComponent|SetMaxWalkSpeed (Variables|Character|GetCharacterMovement) _returnvalue))

(event Custom|MoveToWorldPosition
  (params (Target :type Vector))
  (bind _returnvalue (Math|Vector|MakeVector (.x Target) (.y Target) (.z Target)))
  (bind _returnvalue_2 (AI|GetBlackboard 0))
  (bind _questonmove (Variables|Default|GetQuestOnMove))
  (Utilities|IsValid _questonmove
    (:Is%20Valid
      (Class|EventTriggeredQuestAsset|CompleteQuest _questonmove))
    (:Is%20Not%20Valid
      _))
  (CallFunction|SpawnMovementIndicator _returnvalue)
  (AI|Components|Blackboard|SetValueasVector _returnvalue_2 (Utilities|Name|MakeLiteralName "TargetLocation") _returnvalue)
  (AI|Components|Blackboard|SetValueasEnum _returnvalue_2 (Utilities|Name|MakeLiteralName "EActionEnum") (Utilities|Enum|LiteralenumE_Actions "NewEnumerator3"))
  (AI|Components|Blackboard|ClearValue (AI|GetBlackboard 0) (Utilities|Name|MakeLiteralName "TargetActor"))
  (Utilities|IsValid (Variables|Default|GetTargetActor)
    (:Is%20Valid
      (Class|ToggleAttackIndicator|ToggleIndicator(Message) (Variables|Default|GetTargetActor) self false))
    (:Is%20Not%20Valid
      _))
  (Variables|Default|SetTargetActor 0)
  ;[0 0 0] Play Move Sound
  (if (Variables|Default|GetbIsPrimarySelected)
    (Audio|Components|Audio|Play (Variables|Default|GetMoveSound) 0.0)))

(event Custom|OnSelected
  (params (State :type Boolean))
  (bind _questonselect (Variables|Default|GetQuestOnSelect))
  (bind _questongroupselect (Variables|Default|GetQuestOnGroupSelect))
  (bind _flagindicator (Variables|Default|GetFlagIndicator))
  (if State
    ;[0 0 0] Toggle Decal
    (Rendering|Components|Decal|SetDecalMaterial (Variables|Default|GetDecal) "/Game/Material/M_SelectedUnitGreen.M_SelectedUnitGreen")
    (else
      ;[0 0 0] Toggle Decal
      (Rendering|Components|Decal|SetDecalMaterial (Variables|Default|GetDecal) "/Game/Material/M_SelectedUnit_Decal.M_SelectedUnit_Decal")))
  ;[0 0 0] Toggle Flag
  (Utilities|IsValid _flagindicator
    (:Is%20Valid
      (Rendering|SetActorHiddenInGame _flagindicator (not State)))
    (:Is%20Not%20Valid
      _))
  ;[0 0 0] Check if Primary
  (if (and State (Variables|Default|GetbIsPrimarySelected))
    ;[0 0 0] Play Selection Sound
    (Audio|Components|Audio|Play (Variables|Default|GetSelectedSound) 0.0))
  ;[0 0 0] Quests On Select
  (Utilities|IsValid _questonselect
    (:Is%20Valid
      (Class|EventTriggeredQuestAsset|CompleteQuest _questonselect))
    (:Is%20Not%20Valid
      _))
  (Utilities|IsValid _questongroupselect
    (:Is%20Valid
      (if (and (not (Variables|Default|GetbIsPrimarySelected)) State)
        (Class|EventTriggeredQuestAsset|CompleteQuest _questongroupselect)))))

(event Custom|SetActorTarget
  (params (Target :type Actor%20Object%20Reference))
  (bind _flagindicator (Variables|Default|GetFlagIndicator))
  (if (Utilities|IsValid Target)
    (Utilities|IsValid (Variables|Default|GetTargetActor)
      (:Is%20Valid
        (Class|ToggleAttackIndicator|ToggleIndicator(Message) (Variables|Default|GetTargetActor) self false))
      (:Is%20Not%20Valid
        _))
    (if (Variables|Default|GetbIsPrimarySelected)
      (Audio|Components|Audio|Play (Variables|Default|GetAttackOrder) 0.0))
    (bind _output_get (Variables|Default|SetTargetActor Target))
    (Class|ToggleAttackIndicator|ToggleIndicator(Message) _output_get self true)
    (AI|Components|Blackboard|SetValueasObject (AI|GetBlackboard 0) (Utilities|Name|MakeLiteralName "TargetActor") _output_get)
    (Utilities|IsValid _flagindicator
      (:Is%20Valid
        (Actor|DestroyActor _flagindicator)))))

(event EventBeginPlay
  (bind _questonbuild (Variables|Default|GetQuestOnBuild))
  ;[1 1 1] Updates Movespeed from the UnitStats data asset on a regular basis
  (Utilities|Time|SetTimerbyEvent (delegate Custom|SpeedUpdate) 2.0 true 0.1)
  (if (Variables|Default|GetPlayerUnit)
    (Variables|Default|SetUnitFrameWidget (UserInterface|GetUserWidgetObject (Variables|Default|GetUnitFrame)))
    ;[1 1 1] Hooking up C++ targeting events
    (EventDispatchers|BindEventtoOnNewWorldPositionTarget (delegate Custom|MoveToWorldPosition))
    (EventDispatchers|BindEventtoOnSelectedStateChange (delegate Custom|OnSelected))
    (EventDispatchers|BindEventtoOnNewActorTarget (delegate Custom|SetActorTarget))
    ;[1 1 1] Setting up Ant-on-Ant Collision checks
    (Utilities|Time|SetTimerbyFunctionName 0 "CheckCollisions" (Variables|Default|GetCollisionCheckFrequency) true (Math|Random|RandomFloat))
    (Utilities|IsValid _questonbuild
      (:Is%20Valid
        (Class|EventTriggeredQuestAsset|CompleteQuest _questonbuild)))))

(event EventTick
  (params (DeltaSeconds :type Float%20%28single-precision%29))
  (if (Variables|Default|GetbIsCollidePushing)
    (CallFunction|TickPush DeltaSeconds)))

(event Collision|EventActorBeginOverlap
  (params (OtherActor :type Actor%20Object%20Reference))
  (Utilities|IsValid (Variables|Default|GetFlagIndicator)
    (:Is%20Valid
      (if (== OtherActor (Variables|Default|GetFlagIndicator))
        (Actor|DestroyActor (Variables|Default|GetFlagIndicator))
        (Variables|Default|SetFlagIndicator 0)))))

(event EventDestroyed
  (bind _questondestroy (Variables|Default|GetQuestOnDestroy))
  (bind _flagindicator (Variables|Default|GetFlagIndicator))
  (bind _targetactor (Variables|Default|GetTargetActor))
  (Utilities|IsValid _questondestroy
    (:Is%20Valid
      (Class|EventTriggeredQuestAsset|CompleteQuest _questondestroy))
    (:Is%20Not%20Valid
      _))
  (Utilities|IsValid _flagindicator
    (:Is%20Valid
      (Actor|DestroyActor _flagindicator))
    (:Is%20Not%20Valid
      _))
  (Utilities|IsValid _targetactor
    (:Is%20Valid
      (Class|ToggleAttackIndicator|ToggleIndicator(Message) _targetactor self false))))

(fn ConstructionScript
  (if (not (Variables|Default|GetPlayerUnit))
    (bind _returnvalue (Rendering|Material|CreateDynamicMaterialInstance (Variables|Default|GetDecal) :!class /Script/Engine.DecalComponent))
    (bind _output_get (Variables|Default|SetDecalMaterial _returnvalue))
    (Rendering|Material|SetVectorParameterValue _output_get "DecalColor" "(R=0.770833,G=0.007588,B=0.000000,A=1.000000)" :!class /Script/Engine.MaterialInstanceDynamic)
    (Rendering|SetVisibility (Variables|Default|GetDecal) true false)))

(fn UpdateUnitFrame)

(fn CheckCollisions
  (bind _outactors (Collision|SphereOverlapActors (Transformation|GetActorLocation) (Variables|Default|GetCollisionCheckRadius) (Utilities|Array|MakeArray "ObjectTypeQuery10" "ObjectTypeQuery9" "ObjectTypeQuery11") "BP_UnitBase_C" (Utilities|Array|MakeArray self)))
  (for _array_element _outactors
    (if (< (Math|Vector|Distance(Vector) (Transformation|GetActorLocation _array_element) (Transformation|GetActorLocation)) (* (Variables|Default|GetCollisionCheckRadius) 1.5))
      (Variables|Default|SetbIsCollidePushing true)
      (Variables|Default|SetCollideDirectionNormalized (Math|Vector|Normalize (- (Transformation|GetActorLocation) (Transformation|GetActorLocation _array_element))))
      (Utilities|Time|SetTimerbyFunctionName 0 "DisablePushing" (* (Variables|Default|GetCollisionCheckFrequency) (Variables|Default|GetCollidePushDurationMultiplier)))
      (return))))

(fn DisablePushing
  (Variables|Default|SetbIsCollidePushing false))

(fn TickPush
  (params (DeltaTime :type Float%20%28double-precision%29))
  (Transformation|SetActorLocation (+ (Transformation|GetActorLocation) (/ (* (Variables|Default|GetCollideDirectionNormalized) (Variables|Default|GetCollidePushDistance) DeltaTime) (* (Variables|Default|GetCollisionCheckFrequency) (Variables|Default|GetCollidePushDurationMultiplier)))) false false))

(fn SpawnMovementIndicator
  (params (SpawnLocation :type Vector))
  ;[1 1 1] Destroy old flag before creating new
  (Utilities|IsValid (Variables|Default|GetFlagIndicator)
    (:Is%20Valid
      (Actor|DestroyActor (Variables|Default|GetFlagIndicator)))
    (:Is%20Not%20Valid
      _))
  (bind _returnvalue (Game|SpawnActorfromClass "/Game/Blueprints/3D_UI/VisualFeedback/BP_FlagIndicator.BP_FlagIndicator_C" (Math|Transform|MakeTransform SpawnLocation "0, 0, 0" "1.000000,1.000000,1.000000") "Undefined" 0 0))
  (Variables|Default|SetFlagIndicator _returnvalue))

(fn IsDeletable
  (return true))