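; Base Blueprint for selectable unit buildings that offer a build menu through their BuildingMenu component.
; BeginPlay hands that component to the UnitFrame widget and binds selection changes, which toggle the decal and create or remove a viewport build menu.
; Mouse-follow placement and valid/invalid material swapping are left disconnected.
; PlaceBuilding effectively just sets IsActive, as its material helper is empty and its GameMode cast leads nowhere.
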(event Custom|OnSelected
  (params (State :type Boolean))
  (bind _output_get (Variables|Default|SetIsSelected State))
  ;[1 1 1] Toggeling Decal On/Off
  (Rendering|SetVisibility (Variables|Default|GetDecal) _output_get false)
  (if (Variables|Default|GetIsSelected)
    ;[1 1 1] Toggeling Build Menu On/Off
    (bind _returnvalue (UserInterface|CreateWidget "/Game/UI/UI_BuildMenu.UI_BuildMenu_C"))
    (bind _output_get_2 (Variables|Default|SetBuildMenu _returnvalue))
    (Default|SetOwningBuildingMenuComponent _output_get_2 (Variables|Default|GetBuildingMenu))
    (UserInterface|Viewport|AddtoViewport _output_get_2 0)
    (else
      (Utilities|IsValid (Variables|Default|GetBuildMenu)
        (:Is%20Valid
          (Widget|RemovefromParent (Variables|Default|GetBuildMenu))
          (Variables|Default|SetBuildMenu 0))))))

(event Custom|PlaceBuilding
  (CallFunction|SetMeshMaterials)
  (Variables|Default|SetIsActive true)
  (Utilities|Casting|CastToBP_GP3GameMode (Game|GetGameMode)))

(event EventTick
  (params (DeltaSeconds :type Float%20%28single-precision%29))
  ;[1 1 1] Updating Building Position under mouse
)

(event EventBeginPlay
  (bind _asbp_ui_base_build_menu_widget (Utilities|Casting|CastToBP_UI_BaseBuildMenuWidget (UserInterface|GetUserWidgetObject (Variables|Default|GetUnitFrame))))
  (Default|SetOwningBuildingMenuComponent _asbp_ui_base_build_menu_widget (Variables|Default|GetBuildingMenu))
  (EventDispatchers|BindEventtoOnSelectedStateChange (delegate Custom|OnSelected)))

(fn ConstructionScript
  (|CallParentFunction))

(fn SetCorrectPlacmentMat)

(fn SetMeshMaterials)

(fn SetFalsePlacmentMat)