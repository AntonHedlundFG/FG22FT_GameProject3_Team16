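; BP_UnitWorker is a friendly worker unit that carries food or build material.
; Show and hide events toggle a raspberry or stick component to match the carried resource, and the unit frame widget is updated with the carrying state.
; It registers with BP_GP3GameMode on BeginPlay, then unregisters and returns housing when destroyed.
; Damage goes through the health component, destroying the actor when it is no longer alive.
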(event Custom|ShowResource
  (switch Utilities|FlowControl|Switch|SwitchonEResourceType (Variables|Default|GetCarriedResourceType)
    (:RT_FOOD
      (Rendering|SetVisibility (Variables|Default|GetRasberry) true false))
    (:RT_MATERIAL
      (Rendering|SetVisibility (Variables|Default|GetStick) true false))))

(event Custom|HideResource
  (switch Utilities|FlowControl|Switch|SwitchonEResourceType (Variables|Default|GetCarriedResourceType)
    (:RT_FOOD
      (Rendering|SetVisibility (Variables|Default|GetRasberry) false false))
    (:RT_MATERIAL
      (Rendering|SetVisibility (Variables|Default|GetStick) false false))))

(event EventBeginPlay
  (|CallParentFunction)
  (bind _asui_worker_unit_frame (Utilities|Casting|CastToUI_WorkerUnitFrame (Variables|Default|GetUnitFrameWidget))
    (:then
      (Variables|Default|SetMyUnitFrame _asui_worker_unit_frame))
    (:CastFailed
      _))
  (bind _asbp_gp3game_mode (Utilities|Casting|CastToBP_GP3GameMode (Game|GetGameMode)))
  (Default|RegisterWorker _asbp_gp3game_mode self true))

(event EventDestroyed
  (|CallParentFunction)
  (bind _asbp_gp3game_mode (Utilities|Casting|CastToBP_GP3GameMode (Game|GetGameMode)))
  (Default|RegisterWorker _asbp_gp3game_mode self false)
  (Class|GP3Team16GameModeBase|TryModifyResourceAmount _asbp_gp3game_mode "RT_HOUSING" (Variables|Default|GetHousingReturnOnDeath) false))

(event EventOnDamage
  (params (Damage :type Float%20%28double-precision%29) (AttackingActor :type Actor%20Object%20Reference))
  (bind _bp_healthcomponent (Variables|Default|GetBP_HealthComponent))
  ;[1 1 1] Recieving Damage
  (Default|ChangeHealth _bp_healthcomponent Damage)
  (if (not (Variables|/Game/Blueprints/Health_Damage/BP_HealthComponent.BP_HealthComponent_C|GetisAlive _bp_healthcomponent))
    (Actor|DestroyActor)))

(fn ConstructionScript
  (|CallParentFunction))

(fn UpdateUnitFrame
  (|CallParentFunction)
  (bind _asui_worker_unit_frame (Utilities|Casting|CastToUI_WorkerUnitFrame (Variables|Default|GetUnitFrameWidget)))
  (Default|UpdateFrame _asui_worker_unit_frame (Variables|Default|GetCarryingResource)))