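; BP_UnitRangedWarrior is a friendly ranged unit that extends a parent unit Blueprint and sets its attack speed on BeginPlay.
; Its Projectile event spawns a scaled-up BP_Projectile at the Spawnpoint component, aimed at TargetActor or along the unit's own rotation when no valid target exists.
; It then passes the projectile the distance from unit to target, falling back to a long fixed range without one.
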(event EventBeginPlay
  (|CallParentFunction)
  (Variables|Default|SetAttack%20Speed 1.5))

(event Collision|EventActorBeginOverlap
  (params (OtherActor :type Actor%20Object%20Reference)))

(event EventTick
  (params (DeltaSeconds :type Float%20%28single-precision%29))
  (|CallParentFunction DeltaSeconds) ; This node is disabled and will not be called.\nDrag off pins to build functionality.
)

(event EventProjectile
  (bind _targetactor (Variables|Default|GetTargetActor))
  (bind _targetactor_2 (Variables|Default|GetTargetActor))
  (bind _spawnpoint (Variables|Default|GetSpawnpoint))
  (bind _returnvalue (Transformation|GetWorldLocation _spawnpoint))
  ;[1 1 1] Projectile vfx
  (bind _returnvalue_2 (Game|SpawnActorfromClass "/Game/Blueprints/Projectile/BP_Projectile.BP_Projectile_C" (Math|Transform|MakeTransform _returnvalue (Math|Rotator|SelectRotator (Math|Rotator|FindLookatRotation _returnvalue (Transformation|GetActorLocation _targetactor_2)) (Transformation|GetActorRotation) (Utilities|IsValid _targetactor_2)) "2.000000,2.000000,2.000000") "AlwaysSpawn" 0 0))
  (Utilities|IsValid _targetactor
    (:Is%20Valid
      (Default|SetDistance _returnvalue_2 (Math|Vector|Distance(Vector) (Transformation|GetActorLocation _targetactor) (Transformation|GetActorLocation))))
    (:Is%20Not%20Valid
      (Default|SetDistance _returnvalue_2 1e+04))))

(fn ConstructionScript
  (|CallParentFunction))