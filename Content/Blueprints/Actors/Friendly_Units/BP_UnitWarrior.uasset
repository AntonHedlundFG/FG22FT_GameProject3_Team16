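; BP_UnitWarrior is a friendly combat unit, with tank and ranged (spitter) variants identified by casting.
; It registers by type with the game mode on spawn, then unregisters and returns housing when destroyed.
; Attack turns toward the target, waits, checks range and plays a montage that deals damage on completion, with empty projectile hooks.
; Taking damage adopts the attacker as blackboard target if none exists, updates health UI and destroys dead units.
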(event Custom|Attack
  (bind _targetactor (Variables|Default|GetTargetActor))
  (bind _targetactor_2 (Variables|Default|GetTargetActor))
  ;[1 1 1] Attack
  (Transformation|SetActorRotation (Math|Rotator|MakeRotator 0.0 0.0 (.yaw (Math|Interpolation|RInterpTo (Transformation|GetActorRotation) (Math|Rotator|FindLookatRotation (Transformation|GetActorLocation) (Transformation|GetActorLocation _targetactor_2)) (Utilities|Time|GetWorldDeltaSeconds) 2e+01))))
  (Utilities|FlowControl|Delay (Variables|Default|GetAttack%20Speed))
  (bind _returnvalue (Class|UnitStatsAsset|GetRange (Variables|/Game/Blueprints/Health_Damage/BP_HealthComponent.BP_HealthComponent_C|GetStats%20Asset (Variables|Default|GetBP_HealthComponent))))
  (if (and (Utilities|IsValid _targetactor_2) (<= (Transformation|GetDistanceTo _targetactor_2) _returnvalue))
    (Animation|Montage|PlayMontage (Variables|Character|GetMesh) (Variables|Animation|GetMontage%20to%20Play)
      (:OnCompleted
        (CallFunction|ProjectileHit)
        (bind _returnvalue_2 (Class|UnitStatsAsset|GetDamage (Variables|/Game/Blueprints/Health_Damage/BP_HealthComponent.BP_HealthComponent_C|GetStats%20Asset (Variables|Default|GetBP_HealthComponent))))
        (Utilities|IsValid _targetactor
          (:Is%20Valid
            (Class|BPIDamageable|OnDamage(Message) _targetactor _returnvalue_2 self))))
      (:OnNotifyBegin
        (CallFunction|Projectile)))))

(event Custom|Projectile)

(event Custom|ProjectileHit)

(event EventBeginPlay
  (bind _self self)
  (|CallParentFunction)
  (bind _asbp_gp3game_mode (Utilities|Casting|CastToBP_GP3GameMode (Game|GetGameMode)))
  (bind _asbp_unit_tank (Utilities|Casting|CastToBP_UnitTank _self)
    (:then
      (Default|RegisterTank _asbp_gp3game_mode _asbp_unit_tank true))
    (:CastFailed
      (bind _asbp_unit_ranged_warrior (Utilities|Casting|CastToBP_UnitRangedWarrior _self)
        (:then
          (Default|RegisterSpitter _asbp_gp3game_mode _asbp_unit_ranged_warrior true))
        (:CastFailed
          (Default|RegisterWarrior _asbp_gp3game_mode _self true))))))

(event EventDestroyed
  (bind _self self)
  (|CallParentFunction)
  (bind _asbp_gp3game_mode (Utilities|Casting|CastToBP_GP3GameMode (Game|GetGameMode)))
  (Class|GP3Team16GameModeBase|TryModifyResourceAmount _asbp_gp3game_mode "RT_HOUSING" (Variables|Default|GetHousingReturnOnDeath) false)
  (bind _asbp_unit_tank (Utilities|Casting|CastToBP_UnitTank _self)
    (:then
      (Default|RegisterTank _asbp_gp3game_mode _asbp_unit_tank false))
    (:CastFailed
      (bind _asbp_unit_ranged_warrior (Utilities|Casting|CastToBP_UnitRangedWarrior _self)
        (:then
          (Default|RegisterSpitter _asbp_gp3game_mode _asbp_unit_ranged_warrior false))
        (:CastFailed
          (Default|RegisterWarrior _asbp_gp3game_mode _self false))))))

(event EventOnDamage
  (params (Damage :type Float%20%28double-precision%29) (AttackingActor :type Actor%20Object%20Reference))
  (bind _bp_healthcomponent (Variables|Default|GetBP_HealthComponent))
  (bind _bp_healthcomponent_2 (Variables|Default|GetBP_HealthComponent))
  ;[1 1 1] Change health
  (if (Utilities|IsValid (Variables|Default|GetTargetActor))
    _
    (else
      (bind _output_get (Variables|Default|SetTargetActor AttackingActor))
      (AI|Components|Blackboard|SetValueasObject (AI|GetBlackboard 0) (Utilities|Name|MakeLiteralName "TargetActor") _output_get)))
  (Default|ChangeHealth _bp_healthcomponent_2 Damage)
  (bind _asui_unit_health (Utilities|Casting|CastToUI_UnitHealth (UserInterface|GetUserWidgetObject (Variables|Default|GetUnitFrame))))
  (Default|UpdateHealth _asui_unit_health (Variables|/Game/Blueprints/Health_Damage/BP_HealthComponent.BP_HealthComponent_C|GetCurrentHealth _bp_healthcomponent) (Variables|/Game/Blueprints/Health_Damage/BP_HealthComponent.BP_HealthComponent_C|GetMaxHealth _bp_healthcomponent))
  (if (not (Variables|/Game/Blueprints/Health_Damage/BP_HealthComponent.BP_HealthComponent_C|GetisAlive _bp_healthcomponent_2))
    (Actor|DestroyActor)))

(fn ConstructionScript
  (|CallParentFunction))

(fn UpdateHealthBar)