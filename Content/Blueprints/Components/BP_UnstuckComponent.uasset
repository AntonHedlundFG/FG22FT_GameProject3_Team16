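; Actor component that detects when its owner is off the navmesh and teleports it in an attempt to unstick it.
; A looping timer with randomized initial delay compares the owner's location to its navmesh projection horizontally.
; If they differ, it shifts the owner horizontally along the direction away from the projected point, without sweeping, then rechecks after a shorter delay.
; Optional debug spheres show both locations.
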(event Custom|UnstuckEvent
  (bind _returnvalue (Components|GetOwner))
  (bind _returnvalue_2 (Transformation|GetActorLocation _returnvalue))
  (bind _projectedlocation (AI|Navigation|ProjectPointtoNavigation _returnvalue_2 0 0 "0, 0, 0"))
  (if (Variables|Default|GetbShowDebug) :!label _label
    (Rendering|Debug|DrawDebugSphere _returnvalue_2 5e+01 12 "(R=1.000000,G=0.000000,B=0.048749,A=1.000000)" 5.0)
    (Rendering|Debug|DrawDebugSphere _projectedlocation 5e+01 12 "(R=0.000000,G=0.181463,B=1.000000,A=1.000000)" 5.0))
  (if (>= (Class|KismetMathLibrary|VectorDistanceSquared (* _returnvalue_2 "1.000000,1.000000,0.000000") (* _projectedlocation "1.000000,1.000000,0.000000")) 4e+01)
    (Transformation|SetActorLocation (Components|GetOwner) (+ _returnvalue_2 (* (Math|Vector|Normalize (- _returnvalue_2 _projectedlocation)) "200.000000,200.000000,0.000000")) false true)
    (Utilities|FlowControl|Delay (/ (Variables|Default|GetCheckFrequency) 1e+01))
    (goto _label)))

(event EventBeginPlay
  (bind _checkfrequency (Variables|Default|GetCheckFrequency))
  (Utilities|Time|SetTimerbyEvent (delegate Custom|UnstuckEvent) _checkfrequency true (* _checkfrequency (Math|Random|RandomFloat))))