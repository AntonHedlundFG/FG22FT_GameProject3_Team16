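; Actor component that makes its owner contribute a HousingValue to the game's housing resource while it is in play.
; Shortly after BeginPlay it caches BP_GP3GameMode, updates the housing total and requests an unforced HOUSING resource change.
; On EndPlay it repeats both calls with a value derived from HousingValue, apparently its negation, forcing the resource change.
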(event EventBeginPlay
  (bind _housing_value (Variables|Default|GetHousing%20Value))
  (Utilities|FlowControl|Delay 0.2)
  (bind _asbp_gp3game_mode (Utilities|Casting|CastToBP_GP3GameMode (Game|GetGameMode)))
  (Default|UpdateHousingTotal _asbp_gp3game_mode _housing_value)
  (bind _output_get (Variables|Default|SetGameMode _asbp_gp3game_mode))
  (Class|GP3Team16GameModeBase|TryModifyResourceAmount _output_get "RT_HOUSING" _housing_value false))

(event EventEndPlay
  (params (EndPlayReason :type EEndPlayReason%20Enum :default "Destroyed"))
  (bind _gamemode (Variables|Default|GetGameMode))
  (bind _result (Utilities|NegateInt (Variables|Default|GetHousing%20Value))
    (:%20%20
      (Default|UpdateHousingTotal _gamemode _result)
      (Class|GP3Team16GameModeBase|TryModifyResourceAmount _gamemode "RT_HOUSING" _result true))))