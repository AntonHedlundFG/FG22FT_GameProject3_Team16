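; BP_CursorComponent is a component that sets the mouse cursor shape according to what lies under it.
; It caches player controller 0 on BeginPlay, then runs a complex under-cursor trace every Tick and casts the hit actor.
; Enemy units show crosshairs, while other units and any BuildingActor show a hand.
; Any other hit, or no hit, restores the default cursor.
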(event EventBeginPlay
  ;[0 0 0] Cash Player Controller
  (Variables|Default|SetPController (Game|GetPlayerController 0)))

(event EventTick
  (params (DeltaSeconds :type Float%20%28single-precision%29))
  (bind _pcontroller (Variables|Default|GetPController))
  (bind _pcontroller_2 (Variables|Default|GetPController))
  (bind (_hitresult _returnvalue) (Game|Player|GetHitResultUnderCursorbyChannel _pcontroller_2 "TraceTypeQuery4" true))
  (bind _hitactor (Collision|BreakHitResult _hitresult))
  ;[0 0 0] Get Mouse Over Object
  (if _returnvalue
    ;[0 0 0] Check Mouse Over Units and Buildings
    (bind _asbp_unit_base (Utilities|Casting|CastToBP_UnitBase _hitactor)
      (:then
        (if (Variables|/Script/Units.DirectControlledUnitActor|GetbIsEnemyUnit _asbp_unit_base)
          (Variables|/Script/Engine.PlayerController|SetCurrentMouseCursor _pcontroller "Crosshairs")
          (else
            (Variables|/Script/Engine.PlayerController|SetCurrentMouseCursor _pcontroller "Hand" :!label _label))))
      (:CastFailed
        (Utilities|Casting|CastToBuildingActor _hitactor
          (:then
            (goto _label))
          (:CastFailed
            (Variables|/Script/Engine.PlayerController|SetCurrentMouseCursor _pcontroller "Default" :!label _label_2)))))
    (else
      (goto _label_2))))