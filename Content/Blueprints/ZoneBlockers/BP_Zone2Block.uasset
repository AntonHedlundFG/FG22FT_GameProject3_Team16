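; BP_Zone2Block is a destructible zone blocker that reports as a hostile selectable unit.
; Damage updates its health component and health bar; on death it plays a level sequence, then after a delay spawns a fallen-block actor at a hardcoded transform and destroys itself.
; Destruction completes an optional linked quest.
; An attack indicator stays visible while any tracked attacker remains.
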(event EventDestroyed
  (bind _questondestroy (Variables|Default|GetQuestOnDestroy))
  (Utilities|IsValid _questondestroy
    (:Is%20Valid
      (Class|EventTriggeredQuestAsset|CompleteQuest _questondestroy))))

(event EventToggleIndicator
  (params (SourceActor :type Actor%20Object%20Reference) (Enable :type Boolean))
  (bind _active_attackers (Variables|Default|GetActive%20Attackers))
  (bind _attackindicator (Variables|Default|GetAttackIndicator))
  (Utilities|IsValid SourceActor
    (:Is%20Valid
      (if Enable
        (Utilities|Array|Add _active_attackers SourceActor)
        (Rendering|SetVisibility _attackindicator true false)
        (else
          (Utilities|Array|RemoveItem _active_attackers SourceActor)
          (if (Utilities|Array|IsEmpty _active_attackers)
            (Rendering|SetVisibility _attackindicator false false)))))))

(event EventOnDamage
  (params (Damage :type Float%20%28double-precision%29) (AttackingActor :type Actor%20Object%20Reference))
  (bind _bp_healthcomponent (Variables|Default|GetBP_HealthComponent))
  (bind _bp_healthcomponent_2 (Variables|Default|GetBP_HealthComponent))
  ;[1 1 1] Change Health
  (Default|ChangeHealth _bp_healthcomponent_2 Damage)
  (bind _asui_unit_health (Utilities|Casting|CastToUI_UnitHealth (UserInterface|GetUserWidgetObject (Variables|Default|GetHealthBar))))
  (Default|UpdateHealth _asui_unit_health (Variables|/Game/Blueprints/Health_Damage/BP_HealthComponent.BP_HealthComponent_C|GetCurrentHealth _bp_healthcomponent) (Variables|/Game/Blueprints/Health_Damage/BP_HealthComponent.BP_HealthComponent_C|GetMaxHealth _bp_healthcomponent))
  (if (not (Variables|/Game/Blueprints/Health_Damage/BP_HealthComponent.BP_HealthComponent_C|GetisAlive _bp_healthcomponent_2))
    (Utilities|FlowControl|DoOnce false
      (:Completed
        (bind _outactor (Sequencer|Player|CreateLevelSequencePlayer (Variables|Default|GetLevelSequence)))
        (Sequencer|Player|Play (Variables|/Script/LevelSequence.LevelSequenceActor|GetSequencePlayer _outactor) :!class /Script/MovieScene.MovieSceneSequencePlayer)
        (Utilities|FlowControl|Delay 2.0)
        (Game|SpawnActorfromClass "/Game/Blueprints/ZoneBlockers/BP_ZoneBlock2Down.BP_ZoneBlock2Down_C" (Math|Transform|MakeTransform "-8607.000000,10454.000000,-110.000000" "-2.222000,165.910000,89.000000" "1.500000,1.250000,1.250000") "Undefined" 0 0)
        (Actor|DestroyActor)))))

(fn ConstructionScript)

(fn GetSelectorType
  (return "STT_HOSTILE_UNIT"))