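; Zone 1 blocker actor that acts as a destructible hostile unit, reporting itself as HOSTILEUNIT to selection.
; Damage events update its health component and health bar widget, then destroy it once it is no longer alive.
; An attack indicator stays visible while any tracked attacker remains active.
; When destroyed, it completes its assigned QuestOnDestroy if one is valid.
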(event EventDestroyed
  (bind _questondestroy (Variables|Default|GetQuestOnDestroy))
  (Utilities|IsValid _questondestroy
    (:Is%20Valid
      (Class|EventTriggeredQuestAsset|CompleteQuest _questondestroy))))

(event EventOnDamage
  (params (Damage :type Float%20%28double-precision%29) (AttackingActor :type Actor%20Object%20Reference))
  (bind _bp_healthcomponent (Variables|Default|GetBP_HealthComponent))
  (bind _bp_healthcomponent_2 (Variables|Default|GetBP_HealthComponent))
  ;[1 1 1] Change Health
  (Default|ChangeHealth _bp_healthcomponent_2 Damage)
  (bind _asui_unit_health (Utilities|Casting|CastToUI_UnitHealth (UserInterface|GetUserWidgetObject (Variables|Default|GetHealthBar))))
  (Default|UpdateHealth _asui_unit_health (Variables|/Game/Blueprints/Health_Damage/BP_HealthComponent.BP_HealthComponent_C|GetCurrentHealth _bp_healthcomponent) (Variables|/Game/Blueprints/Health_Damage/BP_HealthComponent.BP_HealthComponent_C|GetMaxHealth _bp_healthcomponent))
  (if (not (Variables|/Game/Blueprints/Health_Damage/BP_HealthComponent.BP_HealthComponent_C|GetisAlive _bp_healthcomponent_2))
    (Actor|DestroyActor)))

(event EventToggleIndicator
  (params (SourceActor :type Actor%20Object%20Reference) (Enable :type Boolean))
  (bind _active_attackers (Variables|Default|GetActive%20Attackers))
  (bind _attackindicator_0 (Variables|Default|GetAttackIndicator_0))
  (Utilities|IsValid SourceActor
    (:Is%20Valid
      (if Enable
        (Utilities|Array|Add _active_attackers SourceActor)
        (Rendering|SetVisibility _attackindicator_0 true false)
        (else
          (Utilities|Array|RemoveItem _active_attackers SourceActor)
          (if (Utilities|Array|IsEmpty _active_attackers)
            (Rendering|SetVisibility _attackindicator_0 false false)))))))

(fn ConstructionScript)

(fn GetSelectorType
  (return "STT_HOSTILE_UNIT"))