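; Health component that tracks current and maximum health, along with alive and full-health flags.
; BeginPlay reads max health from an optional stats asset and starts the component at full health.
; ChangeHealth re-reads that maximum, then applies a signed amount, clamps at zero or max, and updates both flags without broadcasting events.
; SetMaxHealth rescales current health to preserve its ratio whenever the maximum changes.
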(event EventBeginPlay
  (bind _stats_asset (Variables|Default|GetStats%20Asset))
  (Utilities|IsValid _stats_asset
    (:Is%20Valid
      (bind _returnvalue (Class|UnitStatsAsset|GetMaxHealth _stats_asset))
      (Variables|Default|SetMaxHealth _returnvalue))
    (:Is%20Not%20Valid
      _))
  (Variables|Default|SetCurrentHealth (Variables|Default|GetMaxHealth))
  (Variables|Default|SetisAlive true)
  (Variables|Default|SetisFullHealth true))

(fn ChangeHealth
  (params (Change%20amt :type Float%20%28double-precision%29))
  (bind _stats_asset (Variables|Default|GetStats%20Asset))
  ;[1 1 1] Try updating MaxHealth from data asset
  (Utilities|IsValid _stats_asset
    (:Is%20Valid
      (bind _returnvalue (Class|UnitStatsAsset|GetMaxHealth _stats_asset))
      (CallFunction|SetMaxHealth _returnvalue))
    (:Is%20Not%20Valid
      _))
  (if (> Change%20amt 0.0)
    ;[1 1 1] GiveHealth
    (if (>= (+ (Variables|Default|GetCurrentHealth) Change%20amt) (Variables|Default|GetMaxHealth))
      (Variables|Default|SetCurrentHealth (Variables|Default|GetMaxHealth))
      (Variables|Default|SetisFullHealth true)
      (Variables|Default|SetisAlive true)
      (else
        (Variables|Default|SetCurrentHealth (+ (Variables|Default|GetCurrentHealth) Change%20amt))
        (Variables|Default|SetisFullHealth false)
        (Variables|Default|SetisAlive true)))
    (else
      ;[1 1 1] Take Health
      (if (<= (+ (Variables|Default|GetCurrentHealth) Change%20amt) 0.0)
        (Variables|Default|SetCurrentHealth 0.0)
        (Variables|Default|SetisFullHealth false)
        (Variables|Default|SetisAlive false)
        (else
          (Variables|Default|SetCurrentHealth (+ (Variables|Default|GetCurrentHealth) Change%20amt))
          (Variables|Default|SetisFullHealth false)
          (Variables|Default|SetisAlive true))))))

(fn SetMaxHealth
  (params (NewMaxHealth :type Float%20%28double-precision%29))
  (if (== NewMaxHealth (Variables|Default|GetMaxHealth))
    (return)
    (else
      (bind _output_get (LocalVariables|SetRatio (Math|Float|SafeDivide (Variables|Default|GetCurrentHealth) (Variables|Default|GetMaxHealth))))
      (bind _output_get_2 (Variables|Default|SetMaxHealth NewMaxHealth))
      (Variables|Default|SetCurrentHealth (* _output_get_2 _output_get)))))