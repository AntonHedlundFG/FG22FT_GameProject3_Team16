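; Housing building that puffs smoke when it appears and shows a heart effect while a Worker is at the front of its purchase queue.
; BeginPlay spawns a Niagara smoke burst at the actor's location after running the parent logic.
; Tick polls the BuildingMenu queue, and a DoOnce with delays pulses the heart visible for a few seconds, hides it briefly, then re-arms.
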(event EventBeginPlay
  (|CallParentFunction)
  (Niagara|SpawnSystematLocation "/Game/Material/SmokeBurst/NS_SmokeBurst.NS_SmokeBurst" (Transformation|GetActorLocation)))

(event Collision|EventActorBeginOverlap
  (params (OtherActor :type Actor%20Object%20Reference)))

(event EventTick
  (params (DeltaSeconds :type Float%20%28single-precision%29))
  (|CallParentFunction DeltaSeconds)
  (bind _returnvalue (Class|BuildingMenuComponent|GetPurchaseQueue (Variables|Default|GetBuildingMenu)))
  (if (== (Utilities|Array|Get(acopy) _returnvalue) (Variables|Default|GetWorker))
    (Utilities|FlowControl|DoOnce false :!label _label
      (:Completed
        (Development|SetHiddeninGame (Variables|Default|GetNS_Heart) false false)
        (Utilities|FlowControl|Delay 5.0)
        (Development|SetHiddeninGame (Variables|Default|GetNS_Heart) true false)
        (Utilities|FlowControl|Delay 0.2)
        (goto _label Reset)))))

(fn ConstructionScript
  (|CallParentFunction))