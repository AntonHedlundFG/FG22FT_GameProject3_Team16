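; Barracks building that displays animated ant units according to what is first in its purchase queue, with a smoke burst at BeginPlay.
; Tick reads the queue from BuildingMenu and, for a Ranged, Tank or Warrior entry, reveals that type's ants playing looping attack animations.
; Each type has a DoOnce gate and its own hard-coded Delay, after which the ants hide and the gate resets.
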(event EventBeginPlay
  (|CallParentFunction)
  (Niagara|SpawnSystematLocation "/Game/Material/SmokeBurst/NS_SmokeBurst.NS_SmokeBurst" (Transformation|GetActorLocation)))

(event Collision|EventActorBeginOverlap
  (params (OtherActor :type Actor%20Object%20Reference)))

(event EventTick
  (params (DeltaSeconds :type Float%20%28single-precision%29))
  (|CallParentFunction DeltaSeconds)
  (bind _returnvalue (Class|BuildingMenuComponent|GetPurchaseQueue (Variables|Default|GetBuildingMenu)))
  (if (== (Utilities|Array|Get(acopy) _returnvalue) (Variables|Default|GetRanged))
    (Utilities|FlowControl|DoOnce false :!label _label
      (:Completed
        (Development|SetHiddeninGame (Variables|Default|GetAntRanged) false false)
        (Components|Animation|PlayAnimation (Variables|Default|GetAntRanged) "/Game/Art/Characters/AntRanged/AntRangedattack.AntRangedattack" true)
        (Utilities|FlowControl|Delay 15.0)
        (Development|SetHiddeninGame (Variables|Default|GetAntRanged) true false)
        (Utilities|FlowControl|Delay 0.2)
        (goto _label Reset)))
    (elif (== (Utilities|Array|Get(acopy) _returnvalue) (Variables|Default|GetTank))
      (Utilities|FlowControl|DoOnce false :!label _label_2
        (:Completed
          (Development|SetHiddeninGame (Variables|Default|GetAntTank) false false)
          (Components|Animation|PlayAnimation (Variables|Default|GetAntTank) "/Game/Art/Characters/AntTank/Animations/AntTankattack.AntTankattack" true)
          (Utilities|FlowControl|Delay 45.0)
          (Development|SetHiddeninGame (Variables|Default|GetAntTank) true false)
          (Utilities|FlowControl|Delay 0.2)
          (goto _label_2 Reset)))
      (elif (== (Utilities|Array|Get(acopy) _returnvalue) (Variables|Default|GetWarrior))
        (Utilities|FlowControl|DoOnce false :!label _label_3
          (:Completed
            (Development|SetHiddeninGame (Variables|Default|GetAntWarrior1) false false)
            (Components|Animation|PlayAnimation (Variables|Default|GetAntWarrior) "/Game/Art/Characters/AntWarrior/Animations/AntWarriorAttack.AntWarriorAttack" true)
            (Utilities|FlowControl|Delay 1e+01)
            (Development|SetHiddeninGame (Variables|Default|GetAntWarrior) true false)
            (Utilities|FlowControl|Delay 0.2)
            (goto _label_3 Reset)))))))

(fn ConstructionScript
  (|CallParentFunction))