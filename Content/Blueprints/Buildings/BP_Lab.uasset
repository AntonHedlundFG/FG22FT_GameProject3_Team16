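; Lab building that animates its roof and telescope in response to purchases and selection, with a smoke burst on BeginPlay.
; While BuildingMenu's purchase queue has items, Tick plays a roof-rotation timeline whose updates drive a telescope tilt timeline.
; An empty queue stops only the telescope timeline.
; With nothing queued, selection rotates the roof partway and deselection reverses it.
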(event EventBeginPlay
  (|CallParentFunction)
  (Niagara|SpawnSystematLocation "/Game/Material/SmokeBurst/NS_SmokeBurst.NS_SmokeBurst" (Transformation|GetActorLocation)))

(event Collision|EventActorBeginOverlap
  (params (OtherActor :type Actor%20Object%20Reference)))

(event EventTick
  (params (DeltaSeconds :type Float%20%28single-precision%29))
  (|CallParentFunction DeltaSeconds)
  (if (> (Utilities|Array|Length (Variables|/Script/Buildings.BuildingMenuComponent|GetPurchaseQueue (Variables|Default|GetBuildingMenu))) 0)
    (bind _newtrack_0 (Timeline|While%20Building Play)
      (:Update
        (Transformation|SetRelativeRotation (Variables|Default|GetRoof) (Math|Rotator|Lerp(Rotator) "0, 0, 0" "0.000000,120.000000,0.000000" _newtrack_0) false false)
        (bind _newtrack_0_2 (Timeline|Timeline Play)
          (:Update
            (Transformation|SetRelativeRotation (Variables|Default|GetTELESCOPE) (Math|Rotator|Lerp(Rotator) "0, 0, 0" "-30.000000,0.000000,0.000000" _newtrack_0_2) false false)))))
    (else
      (Timeline|Timeline Stop))))

(event EventOnSelected
  (params (State :type Boolean))
  (|CallParentFunction State)
  (if (not (> (Utilities|Array|Length (Variables|/Script/Buildings.BuildingMenuComponent|GetPurchaseQueue (Variables|Default|GetBuildingMenu))) 0))
    (if State
      (bind _newtrack_0 (Timeline|Telescope%20On%20Selected Play)
        (:Update
          (Transformation|SetRelativeRotation (Variables|Default|GetRoof) (Math|Rotator|Lerp(Rotator) "0, 0, 0" "0.000000,56.000000,0.000000" _newtrack_0) false false)))
      (else
        (Timeline|Telescope%20On%20Selected Reverse)))))

(fn ConstructionScript
  (|CallParentFunction))