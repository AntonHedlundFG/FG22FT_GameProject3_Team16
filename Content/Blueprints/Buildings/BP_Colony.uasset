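; BP_Colony is a colony building Blueprint that animates its skeletal mesh when selected and cannot be deleted.
; OnSelected calls the parent, then plays a Timeline that lerps the mesh's relative location vertically upward, reversing it on deselection.
; IsDeletable always returns false, and the construction script only defers to the parent.
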(event EventBeginPlay
  (|CallParentFunction) ; This node is disabled and will not be called.\nDrag off pins to build functionality.
)

(event Collision|EventActorBeginOverlap
  (params (OtherActor :type Actor%20Object%20Reference)))

(event EventTick
  (params (DeltaSeconds :type Float%20%28single-precision%29))
  (|CallParentFunction DeltaSeconds) ; This node is disabled and will not be called.\nDrag off pins to build functionality.
)

(event EventOnSelected
  (params (State :type Boolean))
  (|CallParentFunction State)
  (if State
    (bind _newtrack_0 (Timeline|Timeline Play)
      (:Update
        (Transformation|SetRelativeLocation (Variables|Default|GetSkeletalMesh) (Math|Vector|Lerp(Vector) "-220.000000,-1349.000000,0.000000" "-220.000000,-1349.000000,570.000000" _newtrack_0) false false)))
    (else
      (Timeline|Timeline Reverse))))

(fn ConstructionScript
  (|CallParentFunction))

(fn IsDeletable
  (return false))