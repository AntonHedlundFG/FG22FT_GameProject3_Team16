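; Base building Blueprint that plays a construction sound, completes an optional quest on spawn and reports itself as deletable.
; Selection changes toggle a decal and create or remove the build menu tied to its BuildingMenu component, with a sound on select.
; Tick uses an XOR check to show the progress widget only while selected with queued purchases.
; On destruction it cancels queued purchases as refunds and clears its UI.
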(event OnBeginCursorOver(BoxCollision)
  (params (TouchedComponent :type Primitive%20Component%20Object%20Reference))
  (Development|PrintText "Mouse Over"))

(event Custom|OnSelected
  (params (State :type Boolean))
  ;[0 0 0] Set Selected State
  (bind _output_get (Variables|Default|SetIsSelected State))
  ;[0 0 0] Toggle Decal
  (Rendering|SetVisibility (Variables|Default|GetDecal) _output_get false)
  ;[0 0 0] Check Selection State
  (if (Variables|Default|GetIsSelected)
    ;[0 0 0] Show Build Menu
    (bind _returnvalue (UserInterface|CreateWidget "/Game/UI/UI_BuildMenu.UI_BuildMenu_C"))
    (Default|SetOwningBuildingMenuComponent _returnvalue (Variables|Default|GetBuildingMenu))
    (bind _output_get_2 (Variables|Default|SetBuildMenu _returnvalue))
    (UserInterface|Viewport|AddtoViewport _output_get_2 0)
    ;[0 0 0] Play Selection Sound
    (Audio|Components|Audio|Play (Variables|Default|GetSelectionSound) 0.0)
    (else
      ;[0 0 0] Validate Menu Obj
      (if (Utilities|IsValid (Variables|Default|GetBuildMenu))
        ;[0 0 0] Hide Build Menu
        (Widget|RemovefromParent (Variables|Default|GetBuildMenu))
        (Variables|Default|SetBuildMenu 0)))))

(event Input|EnhancedActionEvents|EnhancedInputActionIA_Delete
  (params (ActionValue :type Boolean) (ElapsedSeconds :type Float%20%28double-precision%29) (TriggeredSeconds :type Float%20%28double-precision%29) (InputAction :type Input%20Action%20Object%20Reference :default "/Game/Settings/Inputs/IA_Delete.IA_Delete"))
  ;[1 1 1] Delete Non-Colony selected buildings
)

(event EventBeginPlay
  (bind _questonbuild (Variables|Default|GetQuestOnBuild))
  ;[0 0 0] Init Menu Widget
  (bind _asbp_ui_base_build_menu_widget (Utilities|Casting|CastToBP_UI_BaseBuildMenuWidget (UserInterface|GetWidget (Variables|Default|GetWidget))))
  (Default|SetOwningBuildingMenuComponent _asbp_ui_base_build_menu_widget (Variables|Default|GetBuildingMenu))
  ;[0 0 0] Bind OnSelected Event
  (EventDispatchers|BindEventtoOnSelectedStateChange (delegate Custom|OnSelected))
  ;[0 0 0] Play Construction Sound
  (Audio|Components|Audio|Play (Variables|Default|GetConstructedSound) 0.0)
  ;[0 0 0] Complete Quest if relevant
  (Utilities|IsValid _questonbuild
    (:Is%20Valid
      (Class|EventTriggeredQuestAsset|CompleteQuest _questonbuild))))

(event EventTick
  (params (DeltaSeconds :type Float%20%28single-precision%29))
  (bind _buildingmenu (Variables|Default|GetBuildingMenu))
  ;[1 1 1] This part handles progress menu visibility.
  ; If the visibility is OFF but should be ON, or vice versa (XOR), toggle the visibility.
  (Utilities|IsValid _buildingmenu
    (:Is%20Valid
      (bind _returnvalue (Class|BuildingMenuComponent|GetPurchaseQueue _buildingmenu))
      (if (Class|KismetMathLibrary|XORBoolean (Variables|Default|GetProgressVisibility) (and (> (Utilities|Array|Length _returnvalue) 0) (Variables|Default|GetIsSelected)))
        (Variables|Default|SetProgressVisibility (not (Variables|Default|GetProgressVisibility)))
        (Rendering|ToggleVisibility (Variables|Default|GetWidget) false)))))

(event EventDestroyed
  (bind _buildingmenu (Variables|Default|GetBuildingMenu))
  (bind _buildmenu (Variables|Default|GetBuildMenu))
  (|CallParentFunction)
  ;[1 1 1] Refund ongoing purchases
  (while (Utilities|Array|IsNotEmpty (Variables|/Script/Buildings.BuildingMenuComponent|GetPurchaseQueue _buildingmenu))
    (Class|BuildingMenuComponent|CancelCurrentPurchase _buildingmenu))
  ;[1 1 1] Remove UI widgets
  (Utilities|IsValid _buildmenu
    (:Is%20Valid
      (Widget|RemovefromParent _buildmenu))
    (:Is%20Not%20Valid
      _))
  (Rendering|SetVisibility (Variables|Default|GetWidget) false false))

(fn ConstructionScript)

(fn IsDeletable
  (return true))