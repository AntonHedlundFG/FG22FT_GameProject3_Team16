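; BP_Projectile is a projectile that spawns a BP_RangedHit effect once it has travelled a set distance.
; It records its start on BeginPlay and checks squared travel distance each Tick against the value that SetDistance stores pre-squared.
; On reaching range it stops movement and delays destruction so the trail is not removed immediately.
; A branch that teleports the actor downward before destruction is never run.
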(event Custom|SpawnProjectileHit
  (Game|SpawnActorfromClass "/Game/Blueprints/Projectile/BP_RangedHit.BP_RangedHit_C" (Math|Transform|MakeTransform (Transformation|GetActorLocation) "0, 0, 0" "1.000000,1.000000,1.000000") "AlwaysSpawn" 0 0))

(event EventBeginPlay
  ;[1 1 1] Establish starting position
  (Variables|Default|SetStartPosition (Transformation|GetActorLocation)))

(event EventTick
  (params (DeltaSeconds :type Float%20%28single-precision%29))
  ;[1 1 1] Check if projectile has travelled far enough
  (if (and (<= (Variables|Default|GetDistance) (Class|KismetMathLibrary|VectorDistanceSquared (Transformation|GetActorLocation) (Variables|Default|GetStartPosition))) (not (Variables|Default|GetbHasExploded)))
    ;[1 1 1] Create a projectile hit effect and stop moving. After a delay, destroy self. We can't destroy self immediately, since the projectile trail is also destroyed.
    (CallFunction|SpawnProjectileHit)
    (Variables|Default|SetbHasExploded true)
    (Components|Movement|StopMovementImmediately (Variables|Default|GetProjectileMovement))
    (Utilities|FlowControl|Delay 2.0)
    (Actor|DestroyActor)))

(fn ConstructionScript)

(fn SetDistance
  (params (Distance :type Float%20%28double-precision%29))
  (Variables|Default|SetDistance (Math|Float|Square Distance)))