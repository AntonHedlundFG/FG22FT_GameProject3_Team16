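; Game mode that tracks the player's workers, warriors, spitters and tanks and creates the resource and keyboard shortcut HUD widgets.
; Register functions add or remove units from per-type lists and push counts to the resource widget, which also receives housing updates.
; Selection functions pass lists to the unit selector component.
; Only workers are filtered by an Idle Blackboard action; the other "SelectIdle" functions select every unit of their type.
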(event Custom|UpdateHousingTotal
  (params (AdditionalHousing :type Integer))
  (Default|UpdateTotalHousing (Variables|Default|GetResourceWidget) AdditionalHousing))

(event EventBeginPlay
  ;[0 0 0] Show UI Resource Menu
  (bind _returnvalue (UserInterface|CreateWidget "/Game/UI/ResourceUi/UI_ResourceMenu.UI_ResourceMenu_C"))
  (UserInterface|Viewport|AddtoViewport _returnvalue 0)
  (Variables|Default|SetResourceWidget _returnvalue)
  (bind _returnvalue_2 (UserInterface|CreateWidget "/Game/UI/UI_KeyboardShortCuts.UI_KeyboardShortCuts_C"))
  (UserInterface|Viewport|AddtoViewport _returnvalue_2 0)
  (Variables|Default|SetKeyboardShortcutUI _returnvalue_2))

(fn ConstructionScript)

(fn RegisterWorker
  (params (Worker :type BP%20Unit%20Worker%20Object%20Reference) (Add :type Boolean))
  (bind _resourcewidget (Variables|Default|GetResourceWidget))
  (bind _activeworkers (Variables|Default|GetActiveWorkers))
  (if Add
    (Utilities|Array|Add _activeworkers Worker)
    (else
      (Utilities|Array|RemoveItem _activeworkers Worker)))
  (Default|UpdateUnitAmount _resourcewidget (Variables|/Game/UI/ResourceUi/UI_ResourceMenu.UI_ResourceMenu_C|GetNumberofWorkers _resourcewidget) (Utilities|Array|Length _activeworkers)))

(fn RegisterWarrior
  (params (Warrior :type BP%20Unit%20Warrior%20Object%20Reference) (Add :type Boolean))
  (bind _activewarriors (Variables|Default|GetActiveWarriors))
  (bind _resourcewidget (Variables|Default|GetResourceWidget))
  (if Add
    (Utilities|Array|Add _activewarriors Warrior)
    (else
      (Utilities|Array|RemoveItem _activewarriors Warrior)))
  (Default|UpdateUnitAmount _resourcewidget (Variables|/Game/UI/ResourceUi/UI_ResourceMenu.UI_ResourceMenu_C|GetNumberOfWarriors _resourcewidget) (Utilities|Array|Length _activewarriors)))

(fn RegisterSpitter
  (params (Spitter :type BP%20Unit%20Ranged%20Warrior%20Object%20Reference) (Add :type Boolean))
  (bind _activespitters (Variables|Default|GetActiveSpitters))
  (bind _resourcewidget (Variables|Default|GetResourceWidget))
  (if Add
    (Utilities|Array|Add _activespitters Spitter)
    (else
      (Utilities|Array|RemoveItem _activespitters Spitter)))
  (Default|UpdateUnitAmount _resourcewidget (Variables|/Game/UI/ResourceUi/UI_ResourceMenu.UI_ResourceMenu_C|GetNumberOfSpitters _resourcewidget) (Utilities|Array|Length _activespitters)))

(fn RegisterTank
  (params (Tank :type BP%20Unit%20Tank%20Object%20Reference) (Add :type Boolean))
  (bind _activetanks (Variables|Default|GetActiveTanks))
  (bind _resourcewidget (Variables|Default|GetResourceWidget))
  (if Add
    (Utilities|Array|Add _activetanks Tank)
    (else
      (Utilities|Array|RemoveItem _activetanks Tank)))
  (Default|UpdateUnitAmount _resourcewidget (Variables|/Game/UI/ResourceUi/UI_ResourceMenu.UI_ResourceMenu_C|GetNumberOfTanks _resourcewidget) (Utilities|Array|Length _activetanks)))

(fn SelectIdleUnits
  (params (UnitList :type Array%20of%20BP%20Unit%20Base%20Object%20References) (OnlyIdle :type Boolean))
  (bind _returnvalue (Class|GP3Team16GameModeBase|GetUnitSelectorComponent))
  (if (and (Utilities|IsValid _returnvalue) (Components|Activation|IsActive _returnvalue))
    (if OnlyIdle
      (for _array_element UnitList
        (switch Utilities|FlowControl|Switch|SwitchonE_Actions (Utilities|Enum|ByteToEnumE_Actions (Class|BlackboardComponent|GetValueasEnum (Variables|/Script/AIModule.AIController|GetBlackboard (AI|GetAIController _array_element)) (Utilities|Name|MakeLiteralName "EActionEnum")))
          (:NewEnumerator2
            (Utilities|Array|Add (LocalVariables|GetIdleUnits) _array_element))))
      (bind _returnvalue_2 (Class|GP3Team16GameModeBase|GetUnitSelectorComponent))
      (Class|UnitSelectorComponent|UnsafeManualSelectList _returnvalue_2 (LocalVariables|GetIdleUnits))
      (else
        (bind _returnvalue_3 (Class|GP3Team16GameModeBase|GetUnitSelectorComponent))
        (Class|UnitSelectorComponent|UnsafeManualSelectList _returnvalue_3 UnitList)))))

(fn SelectIdleWorkers
  (CallFunction|SelectIdleUnits (Variables|Default|GetActiveWorkers) true))

(fn SelectIdleWarriors
  (CallFunction|SelectIdleUnits (Variables|Default|GetActiveWarriors) false))

(fn SelectIdleSpitters
  (CallFunction|SelectIdleUnits (Variables|Default|GetActiveSpitters) false))

(fn SelectIdleTanks
  (CallFunction|SelectIdleUnits (Variables|Default|GetActiveTanks) false))