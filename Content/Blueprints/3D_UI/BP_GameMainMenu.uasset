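; 3D main menu actor that hosts a W_MenuClass widget and moves the player's view between linked menu actors.
; On BeginPlay it binds to the widget's transition callbacks and disables its own collision.
; A widget-supplied index picks from LinkedMenus; TransitionTo shows that menu, enables its collision and eases the view target to it, then resets BlendTime for later blends.
; The transition-from callback hides this menu's widget after a delay.
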(event Custom|TransitionTo
  (params (NewMenu :type BP%20Game%20Main%20Menu%20Object%20Reference))
  (Rendering|SetVisibility (Variables|BP_GameMainMenu_C|GetWidget NewMenu) true false)
  (Collision|SetActorEnableCollision NewMenu true)
  (Game|Player|SetViewTargetwithBlend (Game|GetPlayerController 0) NewMenu (Variables|Default|GetBlend%20Time) "VTBlend_EaseInOut" 2.0 false)
  (Utilities|FlowControl|Delay 0.1)
  (Variables|Default|SetBlend%20Time 2.0))

(event Custom|TransitionToLinkedMenu_Event
  (params (MenuIndex :type Integer))
  (if (Utilities|Array|IsValidIndex (Variables|Default|GetLinkedMenus) MenuIndex)
    (CallFunction|Transitionto (Utilities|Array|Get(acopy) (Variables|Default|GetLinkedMenus) MenuIndex))))

(event Custom|ToggleMenuVisibility
  (Utilities|FlowControl|Delay 2.8)
  (Rendering|SetVisibility (Variables|Default|GetWidget) false false))

(event EventBeginPlay
  (bind _asw_menu_class (Utilities|Casting|CastToW_MenuClass (UserInterface|GetUserWidgetObject (Variables|Default|GetWidget))))
  (EventDispatchers|BindEventtoTransitionfromLinked _asw_menu_class (delegate Custom|ToggleMenuVisibility))
  (EventDispatchers|AssignTransitiontoLinkedMenu _asw_menu_class (delegate Custom|TransitionToLinkedMenu_Event))
  (Collision|SetActorEnableCollision false))

(fn ConstructionScript)