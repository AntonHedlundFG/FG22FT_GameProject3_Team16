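; BP_AntonTestColonyBuilding is a test colony building actor with logic for spawning a test unit.
; Its custom event gets the unit spawn manager from BP_GP3GameMode and calls SpawnUnit with itself as source and a test price data asset.
; A delayed looping timer for that event is left unconnected, so nothing in this graph triggers spawning.
; BeginPlay and the construction script only call their parent versions.
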(event Custom|CustomEvent
  (bind _asbp_gp3game_mode (Utilities|Casting|CastToBP_GP3GameMode (Game|GetGameMode)))
  (bind _returnvalue (Class|GP3Team16GameModeBase|GetUnitSpawnManager _asbp_gp3game_mode))
  (Class|UnitSpawnManager|SpawnUnit _returnvalue self "/Game/Settings/PriceAssets/TestUnitPriceAsset.TestUnitPriceAsset"))

(event EventBeginPlay
  (|CallParentFunction))

(event Collision|EventActorBeginOverlap
  (params (OtherActor :type Actor%20Object%20Reference)))

(event EventTick
  (params (DeltaSeconds :type Float%20%28single-precision%29))
  (|CallParentFunction DeltaSeconds) ; This node is disabled and will not be called.\nDrag off pins to build functionality.
)

(fn ConstructionScript
  (|CallParentFunction))